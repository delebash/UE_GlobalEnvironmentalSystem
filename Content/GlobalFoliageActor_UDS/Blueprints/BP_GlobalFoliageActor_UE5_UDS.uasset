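; Global foliage controller that links Ultra Dynamic Weather to tree and foliage wind, season, health and color variation.
; Construction, editor updates and weather-name changes read the current weather and rerun RunGlobalFoliageActor.
; It takes wind direction from the icon's yaw and scales weather intensity with per-shader adjustments.
; Results go to material parameter collections and back into UDW, optionally syncing the active override volume's wind direction.
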(event Custom|WeatherNameChange
  (params (Weather%20Name :type UDS_Weather_Display_Names%20Enum :default "NewEnumerator0"))
  ;[1 1 1] Setup UDW
  (Variables|UDS-WindWeather|SetCurrent%20Weather%20Name (Utilities|String|EnumtoString Weather%20Name))
  (Variables|UDS-WindWeather|SetCurrent%20Weather (Variables|/Game/UltraDynamicSky/Blueprints/Ultra_Dynamic_Weather.Ultra_Dynamic_Weather_C|GetLocal%20Weather%20State (Variables|UDS-WindWeather|GetUDW)))
  (GlobalWind|RunGlobalFoliageActor))

(event EventEditorUpdate
  ;[1 1 1] Editor Only -- Added Weather Effects Interface to Class Settings.  When you change UDW Weather Type rerun GFA
  (bind _returnvalue (Actor|GetActorOfClass "/Game/UltraDynamicSky/Blueprints/Ultra_Dynamic_Weather.Ultra_Dynamic_Weather_C"))
  (Variables|UDS-WindWeather|SetUDW _returnvalue)
  (Variables|UDS-WindWeather|SetCurrent%20Weather (Variables|/Game/UltraDynamicSky/Blueprints/Ultra_Dynamic_Weather.Ultra_Dynamic_Weather_C|GetWeather (Variables|UDS-WindWeather|GetUDW)))
  (bind _as_string (Default|GetDisplayNameforCurrentWeather (Variables|UDS-WindWeather|GetUDW)))
  (Variables|UDS-WindWeather|SetCurrent%20Weather%20Name _as_string)
  (GlobalWind|RunGlobalFoliageActor))

(event EventBeginPlay
  ;[1 1 1] Setup UDW
  (bind _returnvalue (Actor|GetActorOfClass "/Game/UltraDynamicSky/Blueprints/Ultra_Dynamic_Weather.Ultra_Dynamic_Weather_C"))
  (bind _output_get (Variables|UDS-WindWeather|SetUDW _returnvalue))
  (EventDispatchers|BindEventtoWeatherDisplayNameChanged _output_get (delegate Custom|WeatherNameChange)))

(fn ConstructionScript
  (bind _returnvalue (Actor|GetActorOfClass "/Game/UltraDynamicSky/Blueprints/Ultra_Dynamic_Weather.Ultra_Dynamic_Weather_C"))
  (Variables|UDS-WindWeather|SetUDW _returnvalue)
  (Variables|UDS-WindWeather|SetCurrent%20Weather (Variables|/Game/UltraDynamicSky/Blueprints/Ultra_Dynamic_Weather.Ultra_Dynamic_Weather_C|GetWeather (Variables|UDS-WindWeather|GetUDW)))
  (bind _as_string (Default|GetDisplayNameforCurrentWeather (Variables|UDS-WindWeather|GetUDW)))
  (Variables|UDS-WindWeather|SetCurrent%20Weather%20Name _as_string)
  (GlobalWind|RunGlobalFoliageActor))

(fn RunGlobalFoliageActor
  (bind _icon_sock (Variables|Default|GetIcon_Sock))
  (bind _icon_root (Variables|Default|GetIcon_Root))
  (bind _tree___flip_wind_direction (Variables|GlobalWind|GetTree%20-%20Flip%20Wind%20Direction))
  (bind _udw (Variables|UDS-WindWeather|GetUDW))
  (bind _returnvalue (Transformation|GetWorldRotation _icon_root))
  (bind _yaw (Math|Rotator|BreakRotator _returnvalue))
  ;[1 1 1] Wind
  (Utilities|FlowControl|Sequence
    (:then_0
      (if _tree___flip_wind_direction
        ;[1 1 1] Flipped Icon Function
        (Transformation|SetRelativeRotation _icon_sock "0,180.000000, 0" false false)
        (Transformation|SetRelativeLocation _icon_sock "-220.000000, 0, 0" false false) ; fix location of wind sock center to not intersect with the trees
      )
      (if _tree___flip_wind_direction
        (if (< _yaw 0.0)
          (bind _output_get (Variables|Tree-Wind|SetTree%20-%20Wind%20Direction (+ (* (/ (+ _yaw 3.6e+02) 3.6e+02) -1.0) 1.625)))
          (Rendering|Material|SetScalarParameterValue 0 "Wind Direction" _output_get :!class /Script/Engine.KismetMaterialLibrary)
          (else
            (bind _output_get_2 (Variables|Tree-Wind|SetTree%20-%20Wind%20Direction (+ (* (/ _yaw 3.6e+02) -1.0) 1.625)))
            (Rendering|Material|SetScalarParameterValue 0 "Wind Direction" _output_get_2 :!class /Script/Engine.KismetMaterialLibrary)))
        (elif (< _yaw 0.0)
          (bind _output_get_3 (Variables|Tree-Wind|SetTree%20-%20Wind%20Direction (+ (* (/ (+ _yaw 3.6e+02) 3.6e+02) -1.0) 1.125)))
          (Rendering|Material|SetScalarParameterValue 0 "Wind Direction" _output_get_3 :!class /Script/Engine.KismetMaterialLibrary)
          (else
            (bind _output_get_4 (Variables|Tree-Wind|SetTree%20-%20Wind%20Direction (+ (* (/ _yaw 3.6e+02) -1.0) 1.125)))
            (Rendering|Material|SetScalarParameterValue 0 "Wind Direction" _output_get_4 :!class /Script/Engine.KismetMaterialLibrary))))
      ;[1 1 1] Global Foliage Actor
      (Transformation|SetWorldRotation (Variables|Default|GetIcon_Base) "0, 0, 0" false false)
      (Transformation|SetWorldRotation (Variables|Default|GetIcon_Arrow_Test) (Math|Rotator|MakeRotator 0.0 0.0 (.Yaw (Math|Rotator|BreakRotator (Transformation|GetWorldRotation (Variables|Default|GetIcon_Root))))) false false)
      ;[1 1 1] Wind Parameters
      (Rendering|Material|SetScalarParameterValue 0 "Wind Strength" (Variables|Tree-Wind|GetTree%20-%20Wind%20Strength) :!class /Script/Engine.KismetMaterialLibrary)
      (Rendering|Material|SetScalarParameterValue 0 "Wind Speed" (Variables|Tree-Wind|GetTree%20-%20Wind%20Speed) :!class /Script/Engine.KismetMaterialLibrary)
      (Rendering|Material|SetScalarParameterValue 0 "Wind Tiling" (Variables|Tree-Wind|GetTree%20-%20Wind%20Tiling) :!class /Script/Engine.KismetMaterialLibrary)
      (Rendering|Material|SetScalarParameterValue 0 "Wind Noise" (Variables|Tree-Wind|GetTree%20-%20Wind%20Noise) :!class /Script/Engine.KismetMaterialLibrary)
      ;[1 1 1] Season & Health Parameter
      (Rendering|Material|SetScalarParameterValue 0 "Health" (Variables|Season&Health|GetHealth) :!class /Script/Engine.KismetMaterialLibrary)
      (Rendering|Material|SetScalarParameterValue 0 "Season Strength" (Variables|Season&Health|GetSeason%20Strength) :!class /Script/Engine.KismetMaterialLibrary)
      (Rendering|Material|SetScalarParameterValue 0 "Season Saturation" (Variables|Season&Health|GetSeason%20Saturation) :!class /Script/Engine.KismetMaterialLibrary)
      (Rendering|Material|SetScalarParameterValue 0 "Season Brightness" (Variables|Season&Health|GetSeason%20Brightness) :!class /Script/Engine.KismetMaterialLibrary)
      ;[1 1 1] Color Variation
      (Rendering|Material|SetScalarParameterValue 0 "Variation Tiling" (Variables|ColorVariation|GetVariation%20Tiling) :!class /Script/Engine.KismetMaterialLibrary)
      (Rendering|Material|SetScalarParameterValue 0 "Macro Variation Tiling" (Variables|ColorVariation|GetMacro%20Variation%20Tiling) :!class /Script/Engine.KismetMaterialLibrary)
      (Rendering|Material|SetScalarParameterValue 0 "Random Color Variation" (Variables|ColorVariation|GetRandom%20Color%20Variation%20Amount) :!class /Script/Engine.KismetMaterialLibrary)
      (Rendering|Material|SetScalarParameterValue 0 "Overall Color Variation" (Variables|ColorVariation|GetOverall%20Color%20Variation%20Amount) :!class /Script/Engine.KismetMaterialLibrary))
    (:then_1
      ;[1 1 1] Season & Health For Megascan Foliage
      (Rendering|Material|SetScalarParameterValue "/Game/UltraDynamicSky/Materials/Weather/UltraDynamicWeather_Parameters.UltraDynamicWeather_Parameters" "GFA_Health" (Variables|Season&Health|GetHealth) :!class /Script/Engine.KismetMaterialLibrary)
      (Rendering|Material|SetScalarParameterValue "/Game/UltraDynamicSky/Materials/Weather/UltraDynamicWeather_Parameters.UltraDynamicWeather_Parameters" "GFA_Season_Strength" (Variables|Season&Health|GetSeason%20Strength) :!class /Script/Engine.KismetMaterialLibrary)
      (Rendering|Material|SetScalarParameterValue "/Game/UltraDynamicSky/Materials/Weather/UltraDynamicWeather_Parameters.UltraDynamicWeather_Parameters" "GFA_Season_Saturation" (Variables|Season&Health|GetSeason%20Saturation) :!class /Script/Engine.KismetMaterialLibrary)
      (Rendering|Material|SetScalarParameterValue "/Game/UltraDynamicSky/Materials/Weather/UltraDynamicWeather_Parameters.UltraDynamicWeather_Parameters" "GFA_Season_Brightness" (Variables|Season&Health|GetSeason%20Brightness) :!class /Script/Engine.KismetMaterialLibrary))
    (:then_2
      ;[1 1 1] Set local variabels to parameter collection values
      (Variables|UDS-WindWeather|SetUDS%20-Wind%20Intensity (Variables|/Game/UltraDynamicSky/Blueprints/Weather_Effects/System/UDS_Weather_Settings.UDS_Weather_Settings_C|GetWind%20Intensity (Variables|UDS-WindWeather|GetCurrent%20Weather)))
      (bind _returnvalue_2 (Rendering|Material|GetScalarParameterValue "/Game/UltraDynamicSky/Materials/Weather/UltraDynamicWeather_Parameters.UltraDynamicWeather_Parameters" "Wind Angle" :!class /Script/Engine.KismetMaterialLibrary))
      (Variables|UDS-WindWeather|SetUDS%20-%20Wind%20Direction _returnvalue_2)
      (bind _returnvalue_3 (Rendering|Material|GetScalarParameterValue "/Game/MSPresets/MS_Foliage_Material/MaterialParameterCollection/MPC_GlobalFoliageActor.MPC_GlobalFoliageActor" "Wind Direction" :!class /Script/Engine.KismetMaterialLibrary))
      (Variables|Tree-Wind|SetTree%20-%20Wind%20Direction _returnvalue_3)
      (bind _output_get_5 (Variables|GlobalWind|SetWind%20Direction%20%20Icon%20Rotation (.Yaw (Math|Rotator|BreakRotator (Transformation|GetWorldRotation (Variables|Default|GetIcon_Root))))))
      (Variables|UDS-WindWeather|SetUDS%20-%20Wind%20Direction _output_get_5)
      (Variables|GlobalWind|SetWind%20Intensity%20Multiplied (* (Variables|GlobalWind|GetWind%20Strength%20Multiplier) (Variables|UDS-WindWeather|GetUDS%20-Wind%20Intensity))))
    (:then_3
      ;[1 1 1] Adjust Wind Speeds for difference in UDS, PN Foliage,Trees, and ABS  Wind shaders
      (Variables|PN-Wind|SetPN%20-%20Wind%20Intensity%20Adjusted (+ (Variables|GlobalWind|GetWind%20Intensity%20Multiplied) (Variables|GlobalWind|GetFoliage%20-%20Wind%20Intensity%20Offset)))
      (Variables|Tree-Wind|SetTree%20-%20Wind%20Strength%20Adjusted (+ (* (Variables|GlobalWind|GetWind%20Intensity%20Multiplied) 2.0) (Variables|GlobalWind|GetTrees%20-%20Wind%20Intensity%20Offset)))
      (Variables|AWS-Wind|SetAWS%20-%20Physical%20Wind%20Adjusted (+ (/ (Variables|GlobalWind|GetWind%20Intensity%20Multiplied) 1e+01) (Variables|AWS-Wind|GetAWS%20-%20Physical%20Wind%20Offset)))
      (Variables|AWS-Wind|SetAWS%20-%20Cloth%20Speedtree%20Wind%20Adjusted (+ (/ (Variables|GlobalWind|GetWind%20Intensity%20Multiplied) 1e+01) (Variables|AWS-Wind|GetAWS%20-%20Cloth%20Speedtree%20Wind%20Offset)))
      (Variables|AWS-Wind|SetAWS%20-%20Particle%20Wind%20Adjusted (+ (/ (Variables|GlobalWind|GetWind%20Intensity%20Multiplied) 1e+01) (Variables|AWS-Wind|GetAWS%20-%20Particle%20Wind%20Offset))))
    (:then_4
      ;[1 1 1] Update Parameter Collections
      ;;[0.1995 0.2653 1] PN - Project Nature
      (Rendering|Material|SetScalarParameterValue "/Game/UltraDynamicSky/Materials/Weather/UltraDynamicWeather_Parameters.UltraDynamicWeather_Parameters" "PN Wind Strength" (Variables|PN-Wind|GetPN%20-%20Wind%20Intensity%20Adjusted) :!class /Script/Engine.KismetMaterialLibrary)
      (Rendering|Material|SetScalarParameterValue "/Game/UltraDynamicSky/Materials/Weather/UltraDynamicWeather_Parameters.UltraDynamicWeather_Parameters" "PN Wind Direction" (Variables|GlobalWind|GetWind%20Direction%20%20Icon%20Rotation) :!class /Script/Engine.KismetMaterialLibrary)
      ;;[0.2528 1 0.1602] Trees
      (Rendering|Material|SetScalarParameterValue "/Game/MSPresets/MS_Foliage_Material/MaterialParameterCollection/MPC_GlobalFoliageActor.MPC_GlobalFoliageActor" "Wind Strength" (Variables|Tree-Wind|GetTree%20-%20Wind%20Strength%20Adjusted) :!class /Script/Engine.KismetMaterialLibrary)
      ;;[0.3543 1 0.8079] UDS - UDW
      (Variables|/Game/UltraDynamicSky/Blueprints/Ultra_Dynamic_Weather.Ultra_Dynamic_Weather_C|SetWind%20Direction (Variables|UDS-WindWeather|GetUDW) (Variables|UDS-WindWeather|GetUDS%20-%20Wind%20Direction))
      (Variables|/Game/UltraDynamicSky/Blueprints/Ultra_Dynamic_Weather.Ultra_Dynamic_Weather_C|SetWind%20Intensity (Variables|UDS-WindWeather|GetUDW) (Variables|GlobalWind|GetWind%20Intensity%20Multiplied))
      (Rendering|Material|SetScalarParameterValue "/Game/UltraDynamicSky/Materials/Weather/UltraDynamicWeather_Parameters.UltraDynamicWeather_Parameters" "Wind Angle" (Variables|UDS-WindWeather|GetUDS%20-%20Wind%20Direction) :!class /Script/Engine.KismetMaterialLibrary)
      (Rendering|Material|SetScalarParameterValue "/Game/UltraDynamicSky/Materials/Weather/UltraDynamicWeather_Parameters.UltraDynamicWeather_Parameters" "Wind Intensity" (Variables|GlobalWind|GetWind%20Intensity%20Multiplied) :!class /Script/Engine.KismetMaterialLibrary)
      (if (Variables|GlobalWind|GetSync%20Override%20Volume%20Wind%20Direction)
        (if (Variables|/Game/UltraDynamicSky/Blueprints/Ultra_Dynamic_Weather.Ultra_Dynamic_Weather_C|GetCurrently%20in%20a%20Weather%20Override%20Volume _udw)
          (Variables|/Game/UltraDynamicSky/Blueprints/Weather_Effects/Weather_Override_Volume.Weather_Override_Volume_C|SetWind%20Direction (Variables|/Game/UltraDynamicSky/Blueprints/Ultra_Dynamic_Weather.Ultra_Dynamic_Weather_C|GetCurrent%20Weather%20Override%20Volume _udw) (Variables|UDS-WindWeather|GetUDS%20-%20Wind%20Direction)))))
    (:then_5)
    (:then_6)))

(fn CheckWaveAssetExists
  (params (AssetName :type String) (AssetFolder :type String))
  ;[1 1 1] Check if Wave Asset Exists
  (Variables|Default|SetAsset%20Folder AssetFolder)
  (Variables|Default|SetAsset%20Name AssetName)
  (bind _returnvalue (Class|AssetRegistry|GetAssetbyObjectPath (Class|AssetRegistryHelpers|GetAssetRegistry) (Utilities|String|StringToName (Utilities|String|Append (Utilities|String|Append (Utilities|String|Append (Utilities|String|Append (Variables|Default|GetAsset%20Folder) "/") (Variables|Default|GetAsset%20Name)) ".") (Variables|Default|GetAsset%20Name))) false))
  (if (Class|AssetRegistryHelpers|IsUAsset _returnvalue)
    (return true)
    (else
      (Development|PrintString (Utilities|String|ToString(Name) (Utilities|String|StringToName (Utilities|String|Append (Utilities|String|Append (Utilities|String|Append (Utilities|String|Append (Variables|Default|GetAsset%20Folder) "/") (Variables|Default|GetAsset%20Name)) ".") (Variables|Default|GetAsset%20Name)))) false)
      (Development|PrintString "   Asset Not Found" false))))