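; Template Blueprint of unwired node chains, evidently for copying to enable UE Water and Ambient Wind System support in GlobalFoliageActor_UDS.
; The wind chain passes direction and multipliers to BP_WindZoneBase.
; The water chain loads lake and ocean Gerstner wave assets by weather name, sets wind angle and optional amplitude, recalculates waves, and sets river flowmap speed.
; The ocean branch reuses the "Lake_" prefix and lake sync flag.
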(fn CopyInfo)