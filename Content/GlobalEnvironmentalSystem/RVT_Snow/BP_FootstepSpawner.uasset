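; BP_FootstepSpawner drops BP_Footprint actors along its own path as it moves, in the RVT snow system.
; Tick runs through a 0.2-second Delay, then compares the actor's location with the last stored one and spawns a footprint there only if it has changed.
; Each footprint is rotated to player pawn 0's forward direction with a 90-degree yaw offset.
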(event EventBeginPlay)

(event Collision|EventActorBeginOverlap
  (params (OtherActor :type Actor%20Object%20Reference)))

(event EventTick
  (params (DeltaSeconds :type Float%20%28single-precision%29))
  (bind _returnvalue (Transformation|GetActorLocation))
  (bind _returnvalue_2 (Game|Player|GetPlayerPawn 0))
  (bind _returnvalue_3 (Transformation|GetActorForwardVector _returnvalue_2))
  (bind _returnvalue_4 (Math|Conversions|RotationFromXVector _returnvalue_3))
  (bind (_roll _pitch _yaw) (Math|Rotator|BreakRotator _returnvalue_4))
  (Utilities|FlowControl|Delay 0.2)
  (if (Math|Vector|NotEqual(Vector) _returnvalue (Variables|Default|GetPrevlocation) 0.0001)
    (bind _output_get (Variables|Default|SetPrevlocation _returnvalue))
    (bind _returnvalue_5 (Game|SpawnActorfromClass "/Game/RVT_Snow/BP_Footprint.BP_Footprint_C" (Math|Conversions|ToTransform(Vector) _output_get) "Undefined" 0 0))
    (Transformation|SetActorRotation _returnvalue_5 (Math|Rotator|MakeRotator _roll _pitch (+ _yaw 9e+01)))))

(fn ConstructionScript)