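; Blueprint function library for the Global Environmental System that converts wind direction and speed into a wind force vector.
; GESWindForceVector treats direction as a yaw angle and rotates the X axis by it to get a horizontal heading.
; Magnitude grows non-linearly as a power curve of normalized speed, clamped to a small positive minimum, then multiplied by WindForceScale.
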(fn GESWindForceVector
  (params (Wind%20Direction :type Float%20%28double-precision%29) (Wind%20Speed :type Float%20%28double-precision%29))
  (LocalVariables|SetWind%20Direction%20Local Wind%20Direction)
  (LocalVariables|SetWind%20Speed%20Local Wind%20Speed)
  (return (* (* (Math|Vector|RotateVector "1.000000, 0, 0" (Math|Rotator|MakeRotator 0.0 0.0 (LocalVariables|GetWind%20Direction%20Local))) (Math|Float|Power (/ (Math|Float|Max(Float) (LocalVariables|GetWind%20Speed%20Local) 0.01) 1e+01) 1.5)) (LocalVariables|GetWind%20Force%20Scale))))