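; Helper actor that spawns an Ultra Dynamic Weather radial storm, fades it in and moves it to a target.
; CalcRadialStorm derives direction, distance or target location, and optionally duration from wind speed.
; The construction script runs it to update values without spawning; otherwise it calls SpawnRadialStorm, which also sets UDW's wind direction.
; BeginPlay's test hookup is disconnected, so other Blueprints are expected to call CalcRadialStorm.
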(event EventBeginPlay
  ;[1 1 1] Hookup for quick testing otherwise you will probably have your own bp call Calc Radial Storm when you want to spawn a new storm
)

(fn ConstructionScript
  (bind _returnvalue (Actor|GetActorOfClass "/Game/UltraDynamicSky/Blueprints/Ultra_Dynamic_Weather.Ultra_Dynamic_Weather_C"))
  (Variables|Default|SetUDW _returnvalue)
  (Variables|Default|SetisContructionScript true)
  (CallFunction|CalcRadialStorm))

(fn CalcRadialStorm
  (if (Variables|Default|GetUse%20Direction)
    (Variables|Default|SetForward%20Vector (Math|Vector|GetForwardVector (Math|Rotator|MakeRotator 0.0 0.0 (Variables|Default|GetWind%20Direction))))
    (else
      (Variables|Default|SetForward%20Vector (Math|Vector|GetForwardVector (Math|Rotator|MakeRotator 0.0 0.0 (.yaw (.rotation (Variables|Default|GetSpawn%20Transform))))))))
  (if (Variables|Default|GetUse%20Distance%20or%20Target%20Location)
    (Variables|Default|SetTarget%20Location (+ (.location (Variables|Default|GetSpawn%20Transform)) (* (Variables|Default|GetForward%20Vector) (Variables|Default|GetDistance%20To%20Travel%20In%20CM)))))
  (Variables|Default|SetDistance%20To%20Travel%20In%20CM (Math|Vector|Distance(Vector) (.location (Variables|Default|GetSpawn%20Transform)) (Variables|Default|GetTarget%20Location)))
  (Variables|Default|SetWind%20Direction (.yaw (Math|Conversions|RotationFromXVector (Variables|Default|GetForward%20Vector))))
  (if (Variables|Default|GetUse%20Wind%20Speed%20To%20Calc%20Duration%20Movement)
    (Variables|Default|SetMovement%20Duration (/ (/ (Variables|Default|GetDistance%20To%20Travel%20In%20CM) (Variables|Default|GetDivide%20Distance%20To%20Travel%20By)) (Variables|Default|Get%20Wind%20Speed))))
  (if (not (Variables|Default|GetisContructionScript))
    (CallFunction|SpawnRadialStorm)))

(fn SpawnRadialStorm
  (Variables|/Game/UltraDynamicSky/Blueprints/Ultra_Dynamic_Weather.Ultra_Dynamic_Weather_C|SetWind%20Direction (Variables|Default|GetUDW) (Variables|Default|GetWind%20Direction))
  ;[0.343 0.5016 1] uds radial storm setup
  (bind _returnvalue (Game|SpawnActorfromClass "/Game/UltraDynamicSky/Blueprints/Weather_Effects/Radial_Storm.Radial_Storm_C" (Variables|Default|GetSpawn%20Transform) "Undefined" "MultiplyWithRoot" 0 (Variables|Default|GetStorm%20Weather) (Variables|Default|GetOuter%20Radius) (Variables|Default|GetInner%20Radius%20Fraction) 0))
  (Variables|Default|SetRadial%20Storm _returnvalue)
  (Default|FadeinStorm (Variables|Default|GetRadial%20Storm) (Variables|Default|GetFade%20In%20Duration))
  (Default|MoveStormOverTime (Variables|Default|GetRadial%20Storm) (Variables|Default|GetTarget%20Location) (Variables|Default|GetMovement%20Duration) (Variables|Default|GetFade%20Out%20By%20End%20Of%20Movement) (Variables|Default|GetFade%20Out%20Duration)))