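; Test actor that fast-forwards the Ultra Dynamic Sky calendar to check how the Ultra Dynamic Weather season parameters respond.
; After a startup delay it caches the GES and sky actors, then a looping timer applies the stored date.
; Each tick of that timer then advances the date three days at 10:00, rolling months after day 27 within the same year.
; It prints the advanced date alongside the "UDW Seasons" collection vector.
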(event Custom|ChangeDate
  (Default|SetDateandTime (Variables|Default|GetUDS) (Variables|Default|GetDate%20Time))
  (Variables|Default|SetDate%20Time (Math|DateTime|MakeDateTime (.Year (Math|DateTime|BreakDateTime (Class|KismetMathLibrary|GetDate (Variables|Default|GetDate%20Time)))) (Math|Integer|SelectInt (Math|Integer|SelectInt 1 (+ (.Month (Math|DateTime|BreakDateTime (Class|KismetMathLibrary|GetDate (Variables|Default|GetDate%20Time)))) 1) (> (+ (.Month (Math|DateTime|BreakDateTime (Class|KismetMathLibrary|GetDate (Variables|Default|GetDate%20Time)))) 1) 12)) (.Month (Math|DateTime|BreakDateTime (Class|KismetMathLibrary|GetDate (Variables|Default|GetDate%20Time)))) (> (+ (.Day (Math|DateTime|BreakDateTime (Class|KismetMathLibrary|GetDate (Variables|Default|GetDate%20Time)))) 3) 27)) (Math|Integer|SelectInt 1 (+ (.Day (Math|DateTime|BreakDateTime (Class|KismetMathLibrary|GetDate (Variables|Default|GetDate%20Time)))) 3) (> (+ (.Day (Math|DateTime|BreakDateTime (Class|KismetMathLibrary|GetDate (Variables|Default|GetDate%20Time)))) 3) 27)) 10))
  (bind _returnvalue (Rendering|Material|GetVectorParameterValue "/Game/UltraDynamicSky/Materials/Weather/UltraDynamicWeather_Parameters.UltraDynamicWeather_Parameters" "UDW Seasons" :!class /Script/Engine.KismetMaterialLibrary))
  (Development|PrintText (Utilities|Text|FormatText "[GES_Test] Current date : {d}/{m} - R {R} - G {G} - B {B} - A {A}" (.Day (Math|DateTime|BreakDateTime (Variables|Default|GetDate%20Time))) (.Month (Math|DateTime|BreakDateTime (Variables|Default|GetDate%20Time))) (.R (Math|Color|BreakColor _returnvalue)) (.G (Math|Color|BreakColor _returnvalue)) (.B (Math|Color|BreakColor _returnvalue)) (.A (Math|Color|BreakColor _returnvalue))) true true "(R=0.000000,G=0.660000,B=1.000000,A=1.000000)" 15.0))

(event EventBeginPlay
  (Utilities|FlowControl|Delay (Variables|Default|GetDuration))
  (bind _returnvalue (Actor|GetActorOfClass "/Game/GlobalEnvironmentalSystem/Blueprints/BP_GES.BP_GES_C"))
  (Variables|Default|SetGES _returnvalue)
  (bind _returnvalue_2 (Actor|GetActorOfClass "/Game/UltraDynamicSky/Blueprints/Ultra_Dynamic_Sky.Ultra_Dynamic_Sky_C"))
  (bind _output_get (Variables|Default|SetUDS _returnvalue_2))
  (bind _current_date_and_time (Default|GetCurrentDateandTime _output_get))
  (Variables|Default|SetDate%20Time _current_date_and_time)
  (Utilities|Time|SetTimerbyEvent (delegate Custom|ChangeDate) (Variables|Default|GetTime) true)
  (CallFunction|ChangeDate))

(event Collision|EventActorBeginOverlap
  (params (OtherActor :type Actor%20Object%20Reference)))

(event EventTick
  (params (DeltaSeconds :type Float%20%28single-precision%29)))

(fn ConstructionScript)