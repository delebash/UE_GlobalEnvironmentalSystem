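; Global Environmental System actor that syncs Ultra Dynamic Weather with optional tree, foliage, water and wind integrations.
; RunGlobalEnvironmentalSystem reads weather name, MPC wind intensity and icon or UDW wind direction, then feeds per-integration setters.
; It reruns on construction, editor updates and weather changes, building lake and ocean wave asset names from the weather.
; An optional looping timer switches between winter and non-winter weather to match the season.
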(event Custom|Check%20Season%20Change
  (bind _weather_system (Variables|WeatherSystem|GetWeather%20System))
  (bind _season (Variables|/Game/UltraDynamicSky/Blueprints/Ultra_Dynamic_Weather.Ultra_Dynamic_Weather_C|GetSeason _weather_system))
  ;[0 1 0.2031] Setup UDW
  ;[1 1 1] Change to Winter/Clear Skies weather based on UDS Season Winter or Not Check every hour
  (Utilities|FlowControl|Sequence
    (:then_0
      (Development|PrintString (Utilities|String|ToString(Float) _season))
      (Variables|WeatherSystem|SetisSeasonWinter (Math|Float|InRange(Float) _season (Variables|Season&Health|GetBegin%20UDS%20Winter%20Season) (Variables|Season&Health|GetEnd%20UDS%20Winter%20Season)))
      (bind _as_string (Default|GetDisplayNameforCurrentWeather (Variables|WeatherSystem|GetWeather%20System)))
      (switch string _as_string
        (:Default
          (Variables|WeatherSystem|SetIs%20Weather%20Winter false))
        (:Snow
          (Variables|WeatherSystem|SetIs%20Weather%20Winter true))
        (:Light%20Snow
          (Variables|WeatherSystem|SetIs%20Weather%20Winter true))
        (:Blizzard
          (Variables|WeatherSystem|SetIs%20Weather%20Winter true))))
    (:then_1
      (if (Variables|WeatherSystem|GetisSeasonWinter)
        (if (not (Variables|WeatherSystem|GetIs%20Weather%20Winter))
          (Default|ChangeWeather (Variables|WeatherSystem|GetWeather%20System) (Variables|Season&Health|GetWinter%20Weather%20Type) (Variables|Season&Health|GetChange%20season%20winter%20weather%20delay) true))
        (elif (Variables|WeatherSystem|GetIs%20Weather%20Winter)
          (Default|ChangeWeather (Variables|WeatherSystem|GetWeather%20System) (Variables|Season&Health|GetNon%20Winter%20Weather%20Type) (Variables|Season&Health|GetChange%20season%20winter%20weather%20delay) true))))))

(event Custom|WeatherNameChange
  (params (Weather%20Name :type UDS_Weather_Display_Names%20Enum :default "NewEnumerator0"))
  ;[0 1 0.2031] Setup UDW
  (GlobalWind|RunGlobalEnvironmentalSystem))

(event EventEditorUpdate
  ;[0.9688 0 1] Editor Only -- Added Weather Effects Interface to Class Settings.  When you change UDW Weather Type rerun GFA
  (GlobalWind|RunGlobalEnvironmentalSystem))

(event EventBeginPlay
  ;[0 1 0.2031] Setup UDW
  (Utilities|FlowControl|Sequence
    (:then_0
      (bind _returnvalue (Actor|GetActorOfClass "/Game/UltraDynamicSky/Blueprints/Ultra_Dynamic_Sky.Ultra_Dynamic_Sky_C"))
      (Variables|WeatherSystem|SetSky%20System _returnvalue)
      (bind _returnvalue_2 (Actor|GetActorOfClass "/Game/UltraDynamicSky/Blueprints/Ultra_Dynamic_Weather.Ultra_Dynamic_Weather_C"))
      (EventDispatchers|BindEventtoWeatherDisplayNameChanged _returnvalue_2 (delegate Custom|WeatherNameChange)))
    (:then_1
      (if (Variables|Season&Health|GetSync%20winter%20season%20with%20winter%20weather)
        (Utilities|Time|SetTimerbyEvent (delegate Custom|Check%20Season%20Change) (Variables|Default|GetPoll%20by%20Seconds%20For%20Season%20Change) true)))))

(fn ConstructionScript
  (GlobalWind|RunGlobalEnvironmentalSystem))

(fn RunGlobalEnvironmentalSystem
  (bind _icon_root (Variables|Default|GetIcon_Root))
  (bind _returnvalue (Transformation|GetWorldRotation _icon_root))
  (bind _yaw (Math|Rotator|BreakRotator _returnvalue))
  (Utilities|FlowControl|Sequence
    (:then_0
      ;[0 0.1245 0.2865] GES Settings and Weather System
      ;;[1 0.2812 0] Get Weather System and Current Weather Name and Intensity that is all we need to get regardless of the weather system used.
      (bind _returnvalue_2 (Actor|GetActorOfClass "/Game/UltraDynamicSky/Blueprints/Ultra_Dynamic_Weather.Ultra_Dynamic_Weather_C"))
      (Variables|WeatherSystem|SetWeather%20System _returnvalue_2)
      (bind _as_string (Default|GetDisplayNameforCurrentWeather (Variables|WeatherSystem|GetWeather%20System)))
      (Variables|WeatherSystem|SetWeather%20System%20-%20Weather%20Name _as_string)
      (bind _returnvalue_3 (Rendering|Material|GetScalarParameterValue "/Game/UltraDynamicSky/Materials/Weather/UltraDynamicWeather_Parameters.UltraDynamicWeather_Parameters" "Wind Intensity" :!class /Script/Engine.KismetMaterialLibrary))
      (Variables|WeatherSystem|SetWeather%20System%20-%20Wind%20Intensity (* _returnvalue_3 1e+01)))
    (:then_1
      ;;[1 0 0.3984] Get Windsock Icon Rotation and Set Direction
      (Transformation|SetWorldRotation (Variables|Default|GetIcon_Base) "0, 0, 0" false false)
      (Transformation|SetWorldRotation (Variables|Default|GetIcon_Arrow_Test) (Math|Rotator|MakeRotator 0.0 0.0 _yaw) false false)
      (if (Variables|GlobalWind|GetUse%20UDW%20Wind%20Direction%20instead%20of%20GES)
        (Variables|GlobalWind|SetWind%20Direction%20%20Icon%20Rotation (Variables|/Game/UltraDynamicSky/Blueprints/Ultra_Dynamic_Weather.Ultra_Dynamic_Weather_C|GetCurrent%20Wind%20Direction (Variables|WeatherSystem|GetWeather%20System)))
        (else
          (Variables|GlobalWind|SetWind%20Direction%20%20Icon%20Rotation _yaw))))
    (:then_2
      ;;[0.3458 1 0.4247] Set UDW Wind Direction and Intensity
      (CallFunction|SetUDSUDWGES (Variables|WeatherSystem|GetWeather%20System) (Variables|GlobalWind|GetSync%20Override%20Volume%20Wind%20Direction) (Variables|WeatherSystem|GetWeather%20System%20-%20Wind%20Intensity) (Variables|GlobalWind|GetWind%20Strength%20Multiplier) (Variables|GlobalWind|GetWind%20Direction%20%20Icon%20Rotation)))
    (:then_3
      ;[0.3906 0 0.00444] Add Systems To Integrate
      ;;[0.1437 1 0.2378] Enable MS Trees
      (if (Variables|EnableSystems|GetEnable%20MS%20Trees)
        (CallFunction|SetMSTreesGES (Variables|GlobalWind|GetFlip%20MS%20Trees%20Wind%20Direction) (Variables|WeatherSystem|GetWeather%20System%20-%20Wind%20Intensity) (/ (Variables|GlobalWind|GetWind%20Strength%20Multiplier) 0.5) (Variables|GlobalWind|GetTrees%20-%20Wind%20Intensity%20Offset) (Variables|GlobalWind|GetWind%20Direction%20%20Icon%20Rotation) (Variables|Default|GetIcon_Sock) (Variables|MSTreeWind|GetTree%20-%20Wind%20Speed) (Variables|MSTreeWind|GetTree%20-%20Wind%20Tiling) (Variables|MSTreeWind|GetTree%20-%20Wind%20Noise))))
    (:then_4
      ;;[0.2183 1 0.1567] Enable MS Trees Health Seasons and Color Variation
      (if (Variables|EnableSystems|GetEnable%20MS%20Trees%20Health%20and%20Seasons)
        (CallFunction|SetMSTreesHealthSeasonsGES (Variables|Season&Health|GetHealth) (Variables|Season&Health|GetSeason%20Strength) (Variables|Season&Health|GetSeason%20Saturation) (Variables|Season&Health|GetSeason%20Brightness) (Variables|MSTreeColorVariation|GetVariation%20Tiling) (Variables|MSTreeColorVariation|GetMacro%20Variation%20Tiling) (Variables|MSTreeColorVariation|GetRandom%20Color%20Variation%20Amount) (Variables|MSTreeColorVariation|GetOverall%20Color%20Variation%20Amount))))
    (:then_5
      ;;[0.2059 1 0.9403] Enable Project Nature Wind
      (if (Variables|EnableSystems|GetEnable%20Project%20Nature)
        (CallFunction|SetProjectNatureGES (Variables|WeatherSystem|GetWeather%20System%20-%20Wind%20Intensity) (Variables|GlobalWind|GetWind%20Strength%20Multiplier) (Variables|GlobalWind|GetFoliage%20-%20Wind%20Intensity%20Offset) (Variables|GlobalWind|GetWind%20Direction%20%20Icon%20Rotation))))
    (:then_6
      ;;[1 1 1] Enable Foliage Health and Season
      (if (Variables|EnableSystems|GetEnable%20Foliage%20Health%20and%20Season)
        (CallFunction|SetFoliageHealthandSeasonGES (Variables|Season&Health|GetHealth) (Variables|Season&Health|GetSeason%20Strength) (Variables|Season&Health|GetSeason%20Saturation) (Variables|Season&Health|GetSeason%20Brightness))))
    (:then_7
      ;;[1 1 1] Enable Foliage Interaction Wind System
      (if (Variables|EnableSystems|GetEnable%20Foliage%20Wind%20System)
        (CallFunction|SetFoliageInteractionWindSystemGES (Variables|WeatherSystem|GetWeather%20System%20-%20Wind%20Intensity) (Variables|GlobalWind|GetWind%20Strength%20Multiplier) (Variables|GlobalWind|GetFoliage%20-%20Wind%20Intensity%20Offset) (Variables|GlobalWind|GetWind%20Direction%20%20Icon%20Rotation))))
    (:then_8
      ;;[0.03105 0.02241 0.6146] Enable UE Water
      (if (Variables|EnableSystems|GetEnable%20UE%20Water)
        (Utilities|FlowControl|Sequence
          (:then_0
            (Variables|UEWaterSystem|SetLake%20Wave%20Asset%20Name (Utilities|String|Append "Lake_" (Variables|WeatherSystem|GetWeather%20System%20-%20Weather%20Name)))
            (Variables|UEWaterSystem|SetOcean%20Wave%20Asset%20Name (Utilities|String|Append "Ocean_" (Variables|WeatherSystem|GetWeather%20System%20-%20Weather%20Name))))
          (:then_1
            (CallFunction|SetUEWaterGES (Variables|UEWaterSystem|GetEnable%20Lake) (Variables|UEWaterSystem|GetSync%20Lake%20To%20Weather) (Variables|UEWaterSystem|GetEnable%20Lake%20Wave%20Override) (Variables|UEWaterSystem|GetLake%20-%20Override%20Max%20Amplitude) (Variables|UEWaterSystem|GetEnable%20Ocean) (Variables|UEWaterSystem|GetSync%20Ocean%20To%20Weather) (Variables|UEWaterSystem|GetEnable%20Ocean%20Wave%20Override) (Variables|UEWaterSystem|GetOcean%20-%20Override%20Max%20Amplitude) (Variables|UEWaterSystem|GetEnable%20River) (Variables|UEWaterSystem|GetRiver%20Wind%20Direction%20and%20Velocity) (Variables|UEWaterSystem|GetLake%20Wave%20Asset%20Name) (Variables|UEWaterSystem|GetOcean%20Wave%20Asset%20Name) (Variables|UEWaterSystem|GetWave%20Asset%20Folder))))))
    (:then_9
      ;;[1 1 1] Enable SpeedTree
      (if (Variables|EnableSystems|GetEnable%20SpeedTree)
        (CallFunction|SetSpeedTreeGES (Variables|WeatherSystem|GetWeather%20System%20-%20Wind%20Intensity) (Variables|GlobalWind|GetWind%20Strength%20Multiplier) (Variables|GlobalWind|GetTrees%20-%20Wind%20Intensity%20Offset) (Variables|GlobalWind|GetWind%20Direction%20%20Icon%20Rotation))))
    (:then_10
      ;;[1 1 1] Enable Brushify
      (if (Variables|EnableSystems|GetEnable%20Brushify)
        (CallFunction|SetBrushifyGES (Variables|WeatherSystem|GetWeather%20System%20-%20Wind%20Intensity) (/ (Variables|GlobalWind|GetWind%20Strength%20Multiplier) 9.0) (Variables|GlobalWind|GetFoliage%20-%20Wind%20Intensity%20Offset) (Variables|GlobalWind|GetTrees%20-%20Wind%20Intensity%20Offset))))
    (:then_11
      ;;[0.9164 1 0.2395] Enable Ambient Wind System
      (if (Variables|EnableSystems|GetEnable%20Ambient%20Wind%20System)
        (CallFunction|SetAmbientWindSystemGES (Variables|WeatherSystem|GetWeather%20System%20-%20Wind%20Intensity) (Variables|GlobalWind|GetWind%20Strength%20Multiplier) (Variables|AWSWind|GetAWS%20-%20Particle%20Wind%20Offset) (Variables|AWSWind|GetAWS%20-%20Cloth%20Speedtree%20Wind%20Offset) (Variables|AWSWind|GetAWS%20-%20Physical%20Wind%20Offset) (Variables|GlobalWind|GetWind%20Direction%20%20Icon%20Rotation))))
    (:then_12
      ;;[1 1 1] Enable Particle Wind System
      (if (Variables|EnableSystems|GetEnable%20Particles_Wind_Control_System)
        (CallFunction|SetParticlesWindControlSystemGES (Variables|WeatherSystem|GetWeather%20System%20-%20Wind%20Intensity) (Variables|/Game/UltraDynamicSky/Blueprints/Ultra_Dynamic_Weather.Ultra_Dynamic_Weather_C|GetCurrent%20Wind%20Direction (Variables|WeatherSystem|GetWeather%20System)) (Variables|ParticleWindSystem|GetParticle%20Wind%20Strength%20Factor))))))

(fn CheckWaveAssetExists
  (params (AssetName :type String) (AssetFolder :type String))
  ;[1 0.2109 0] Check if Wave Asset Exists
  (Variables|Misc|SetAsset%20Folder AssetFolder)
  (Variables|Misc|SetAsset%20Name AssetName)
  (bind _returnvalue (Class|AssetRegistry|GetAssetbyObjectPath (Class|AssetRegistryHelpers|GetAssetRegistry) (Utilities|String|StringToName (Utilities|String|Append (Utilities|String|Append (Utilities|String|Append (Utilities|String|Append (Variables|Misc|GetAsset%20Folder) "/") (Variables|Misc|GetAsset%20Name)) ".") (Variables|Misc|GetAsset%20Name))) false))
  (if (Class|AssetRegistryHelpers|IsUAsset _returnvalue)
    (return true)
    (else
      (Development|PrintString (Utilities|String|ToString(Name) (Utilities|String|StringToName (Utilities|String|Append (Utilities|String|Append (Utilities|String|Append (Utilities|String|Append (Variables|Misc|GetAsset%20Folder) "/") (Variables|Misc|GetAsset%20Name)) ".") (Variables|Misc|GetAsset%20Name)))) false)
      (Development|PrintString "   Asset Not Found" false))))