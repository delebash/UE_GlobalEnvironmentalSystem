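; Blueprint function for the Global Environmental System's foliage health and season integration, setting the health and seasonal look of foliage.
; It writes health plus season strength, saturation and brightness into the "MS Foliage" scalar parameters of the MPC_GES Material Parameter Collection.
; Values pass through unmodified, so any material reading that collection picks up the change globally without per-instance updates.
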(fn SetFoliageHealthandSeasonGES
  (params (Health :type Float%20%28double-precision%29) (Season%20Strength :type Float%20%28double-precision%29) (Season%20Saturation :type Float%20%28double-precision%29) (Season%20Brightness :type Float%20%28double-precision%29))
  (LocalVariables|SetSeason%20Brightness%20Local Season%20Brightness)
  (LocalVariables|SetSeason%20Saturation%20Local Season%20Saturation)
  (LocalVariables|SetSeason%20Strength%20Local Season%20Strength)
  (LocalVariables|SetHealth%20Local Health)
  ;[0.2422 0 1] Foliage Season & Health Parameter
  (Rendering|Material|SetScalarParameterValue 0 "/Game/GlobalEnvironmentalSystem/MaterialParameterCollection/MPC_GES.MPC_GES" "MS Foliage Health" (LocalVariables|GetHealth%20Local) :!class /Script/Engine.KismetMaterialLibrary)
  (Rendering|Material|SetScalarParameterValue 0 "/Game/GlobalEnvironmentalSystem/MaterialParameterCollection/MPC_GES.MPC_GES" "MS Foliage Season Strength" (LocalVariables|GetSeason%20Strength%20Local) :!class /Script/Engine.KismetMaterialLibrary)
  (Rendering|Material|SetScalarParameterValue 0 "/Game/GlobalEnvironmentalSystem/MaterialParameterCollection/MPC_GES.MPC_GES" "MS Foliage Season Saturation" (LocalVariables|GetSeason%20Saturation%20Local) :!class /Script/Engine.KismetMaterialLibrary)
  (Rendering|Material|SetScalarParameterValue 0 "/Game/GlobalEnvironmentalSystem/MaterialParameterCollection/MPC_GES.MPC_GES" "MS Foliage Season Brightness" (LocalVariables|GetSeason%20Brightness%20Local) :!class /Script/Engine.KismetMaterialLibrary))