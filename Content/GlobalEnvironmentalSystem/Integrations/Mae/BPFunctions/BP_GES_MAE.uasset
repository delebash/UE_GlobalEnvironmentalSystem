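; BP_GES_MAE bridges the Global Environmental System's wind to MAE trees through the MPC_GlobalFoliageActor parameter collection.
; SetMAEGES converts changed wind direction from degrees into an offset material value, optionally flipping and repositioning the wind sock icon.
; On speed changes, it matches a preset array by weather type or intensity range, writing strength, speed, tiling and noise only when strength differs.
; Without the array, wind intensity directly drives strength.
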(fn SetMAEGES
  (params (Weather%20System%20-%20Wind%20Intensity :type Float%20%28double-precision%29) (Wind%20Strength%20Multiplier :type Float%20%28double-precision%29) (Wind%20Direction :type Float%20%28double-precision%29) (Wind%20Speed%20Array :type Array%20of%20GES%20MAE%20Wind%20Speed%20Struct%20Structures) (Weather%20Display%20Name%20Enum :type GES_UDS_Weather_Display_Names%20Enum :default "NewEnumerator15") (Use%20Windspeed%20Array :type Boolean) (Wind%20Direction%20Change :type Boolean) (Flip%20Tree%20Direction :type Boolean) (Icon%20Stock :type Static%20Mesh%20Component%20Object%20Reference) (Wind%20Speed%20Change :type Boolean))
  (LocalVariables|SetWind%20Speed%20Change%20Local Wind%20Speed%20Change)
  (LocalVariables|SetFlip%20Tree%20Direction%20Local Flip%20Tree%20Direction)
  (LocalVariables|SetIcon_Sock%20Local Icon%20Stock)
  (LocalVariables|SetUse%20Windspeed%20Array%20Local Use%20Windspeed%20Array)
  (LocalVariables|SetWeather%20Display%20Name%20Enum%20Local Weather%20Display%20Name%20Enum)
  (LocalVariables|SetWind%20Speed%20Array%20Local Wind%20Speed%20Array)
  (LocalVariables|SetWind%20Direction%20Local Wind%20Direction)
  (LocalVariables|SetWind%20Strength%20Multiplier%20Local Wind%20Strength%20Multiplier)
  (LocalVariables|SetWeather%20System%20Wind%20Intensity%20Local Weather%20System%20-%20Wind%20Intensity)
  (LocalVariables|SetWind%20Direction%20Change%20Local Wind%20Direction%20Change)
  (Utilities|FlowControl|Sequence
    (:then_0
      (if (LocalVariables|GetWind%20Direction%20Change%20Local)
        (Utilities|FlowControl|Sequence
          (:then_0
            ;[0 0.3906 1] Set MAE Trees Direction
            (if (LocalVariables|GetFlip%20Tree%20Direction%20Local)
              ;[1 0.8906 0] MAE Trees Flipped Icon Function
              (Transformation|SetRelativeRotation (LocalVariables|GetIcon_Sock%20Local) "0,180.000000, 0" false false)
              (Transformation|SetRelativeLocation (LocalVariables|GetIcon_Sock%20Local) "-220.000000, 0, 0" false false) ; fix location of wind sock center to not intersect with the trees
            )
            (if true
              (if (< (LocalVariables|GetWind%20Direction%20Local) 0.0)
                (LocalVariables|SetTree%20Wind%20Direction%20Local (+ (* (/ (+ (LocalVariables|GetWind%20Direction%20Local) 3.6e+02) 3.6e+02) -1.0) 1.625))
                (else
                  (LocalVariables|SetTree%20Wind%20Direction%20Local (+ (* (/ (LocalVariables|GetWind%20Direction%20Local) 3.6e+02) -1.0) 1.625))))
              (elif (< (LocalVariables|GetWind%20Direction%20Local) 0.0)
                (LocalVariables|SetTree%20Wind%20Direction%20Local (+ (* (/ (+ (LocalVariables|GetWind%20Direction%20Local) 3.6e+02) 3.6e+02) -1.0) 1.125))
                (else
                  (LocalVariables|SetTree%20Wind%20Direction%20Local (+ (* (/ (LocalVariables|GetWind%20Direction%20Local) 3.6e+02) -1.0) 1.125))))))
          (:then_1
            ;[1 1 1] Wind Direction
            (Rendering|Material|SetScalarParameterValue 0 "/Game/MAEOakForest/Materials/MaterialParameterCollection/MPC_GlobalFoliageActor.MPC_GlobalFoliageActor" "Wind Direction" (LocalVariables|GetTree%20Wind%20Direction%20Local) :!class /Script/Engine.KismetMaterialLibrary)))))
    (:then_1
      (if (LocalVariables|GetWind%20Speed%20Change%20Local)
        ;[1 1 1] Weather Type Wind Speed Array
        (if (LocalVariables|GetUse%20Windspeed%20Array%20Local)
          (bind _array_element (Utilities|Array|ForEachLoopwithBreak (LocalVariables|GetWind%20Speed%20Array%20Local) :!label _label)
            (:LoopBody
              (LocalVariables|SetArray%20Wind%20Noise (.windnoise _array_element))
              (LocalVariables|SetArray%20Wind%20Speed (.windspeed _array_element))
              (LocalVariables|SetArray%20Wind%20Tiling (.windtiling _array_element))
              (LocalVariables|SetArray%20Wind%20Strength (.windstrength _array_element))
              (LocalVariables|SetArray%20Wind%20Speed%20Less%20Than (.windspeedlessthanequal _array_element))
              (LocalVariables|SetArray%20Wind%20Speed%20Greater%20Than (.windspeedgreaterthanequal _array_element))
              (LocalVariables|SetArray%20Use%20Multiplier (.usemultplier? _array_element))
              (bind _output_get (LocalVariables|SetArray%20Use%20Display%20Name (.useweathernameorwindspeed _array_element)))
              (LocalVariables|SetArray%20Weather%20Display%20Name%20Type%20Enum (.weathertypeenum _array_element))
              (if _output_get
                (if (Utilities|Enum|Equal(Enum) (LocalVariables|GetWeather%20Display%20Name%20Enum%20Local) (LocalVariables|GetArray%20Weather%20Display%20Name%20Type%20Enum))
                  (if (LocalVariables|GetArray%20Use%20Multiplier) :!label _label_2
                    (LocalVariables|SetArray%20Wind%20Strength (* (LocalVariables|GetWind%20Strength%20Multiplier%20Local) (LocalVariables|GetArray%20Wind%20Strength))))
                  (bind _returnvalue (Rendering|Material|GetScalarParameterValue 0 "/Game/MAEOakForest/Materials/MaterialParameterCollection/MPC_GlobalFoliageActor.MPC_GlobalFoliageActor" "Wind Strength" :!class /Script/Engine.KismetMaterialLibrary))
                  (if (!= _returnvalue (LocalVariables|GetArray%20Wind%20Strength))
                    ;[0.875 0 1] MAE Tree Wind Parameters
                    (Rendering|Material|SetScalarParameterValue 0 "/Game/MAEOakForest/Materials/MaterialParameterCollection/MPC_GlobalFoliageActor.MPC_GlobalFoliageActor" "Wind Strength" (LocalVariables|GetArray%20Wind%20Strength) :!class /Script/Engine.KismetMaterialLibrary)
                    (Rendering|Material|SetScalarParameterValue 0 "/Game/MAEOakForest/Materials/MaterialParameterCollection/MPC_GlobalFoliageActor.MPC_GlobalFoliageActor" "Wind Speed" (LocalVariables|GetArray%20Wind%20Speed) :!class /Script/Engine.KismetMaterialLibrary)
                    (Rendering|Material|SetScalarParameterValue 0 "/Game/MAEOakForest/Materials/MaterialParameterCollection/MPC_GlobalFoliageActor.MPC_GlobalFoliageActor" "Wind Tiling" (LocalVariables|GetArray%20Wind%20Tiling) :!class /Script/Engine.KismetMaterialLibrary)
                    (Rendering|Material|SetScalarParameterValue 0 "/Game/MAEOakForest/Materials/MaterialParameterCollection/MPC_GlobalFoliageActor.MPC_GlobalFoliageActor" "Wind Noise" (LocalVariables|GetArray%20Wind%20Noise) :!class /Script/Engine.KismetMaterialLibrary)
                    (goto _label Break)))
                (elif (Math|Float|InRange(Float) (LocalVariables|GetWeather%20System%20Wind%20Intensity%20Local) (LocalVariables|GetArray%20Wind%20Speed%20Greater%20Than) (LocalVariables|GetArray%20Wind%20Speed%20Less%20Than))
                  (goto _label_2)))))
          (else
            ;[1 1 1] Multiplier for Direct
            (if (LocalVariables|GetArray%20Use%20Multiplier)
              (LocalVariables|SetWeather%20System%20Wind%20Intensity%20Local (* (LocalVariables|GetWind%20Strength%20Multiplier%20Local) (LocalVariables|GetWeather%20System%20Wind%20Intensity%20Local))))
            ;[0.875 0 1] MAE Tree Wind Parameters
            (Rendering|Material|SetScalarParameterValue 0 "/Game/MAEOakForest/Materials/MaterialParameterCollection/MPC_GlobalFoliageActor.MPC_GlobalFoliageActor" "Wind Strength" (LocalVariables|GetWeather%20System%20Wind%20Intensity%20Local) :!class /Script/Engine.KismetMaterialLibrary)))))))