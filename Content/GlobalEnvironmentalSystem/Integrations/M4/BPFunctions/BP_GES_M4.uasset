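; Blueprint integration between the Global Environmental System (GES) and M4, writing wind values to the AW_MPC5N material parameter collection.
; SetM4GES takes weather wind intensity, multiplier, offset and direction, then computes an adjusted intensity.
; That result is unused: Wind Strength and Wind Speed are set to a hardcoded 100.
; The Wind Direction and Wind Noise Speed writes are disconnected, so they never run.
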(fn SetM4GES
  (params (Weather%20System%20-%20Wind%20Intensity :type Float%20%28double-precision%29) (Wind%20Strength%20Multiplier :type Float%20%28double-precision%29) (Wind%20Intensity%20Offset :type Float%20%28double-precision%29) (Wind%20Direction :type Float%20%28double-precision%29))
  (LocalVariables|SetWind%20Direction%20Local Wind%20Direction)
  (LocalVariables|SetWind%20Intensity%20Offset%20Local Wind%20Intensity%20Offset)
  (LocalVariables|SetWind%20Strength%20Multiplier%20Local Wind%20Strength%20Multiplier)
  (LocalVariables|SetWeather%20System%20Wind%20Intensity%20Local Weather%20System%20-%20Wind%20Intensity)
  (Utilities|FlowControl|Sequence
    (:then_0
      ;[0 0.01562 1] Adjust Wind Speed
      (LocalVariables|SetWind%20Intensity%20Adjusted%20Local (+ (* (LocalVariables|GetWeather%20System%20Wind%20Intensity%20Local) (LocalVariables|GetWind%20Strength%20Multiplier%20Local)) (LocalVariables|GetWind%20Intensity%20Offset%20Local))))
    (:then_1
      ;[0.875 0 1] M4 Wind Parameters
      (Rendering|Material|SetScalarParameterValue 0 "/Game/M4/Blueprints/SystemResources/Trails/MPCs/AW_MPC5N.AW_MPC5N" "Wind Strength" 1e+02 :!class /Script/Engine.KismetMaterialLibrary)
      (Rendering|Material|SetScalarParameterValue 0 "/Game/M4/Blueprints/SystemResources/Trails/MPCs/AW_MPC5N.AW_MPC5N" "Wind Speed" 1e+02 :!class /Script/Engine.KismetMaterialLibrary))))