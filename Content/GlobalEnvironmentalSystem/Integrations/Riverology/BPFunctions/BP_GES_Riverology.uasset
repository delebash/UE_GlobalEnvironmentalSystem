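; Global Environmental System integration function that drives Riverology water waves from weather wind by writing to the MPC_Riverology material parameter collection.
; In array mode it searches wind-speed entries by weather type or intensity range, then applies the first non-multiplier match's full wave preset.
; Otherwise it scales and offsets wind intensity into Global Amplitude and Global Speed.
; The wind direction input is unused, and entries flagged to use a multiplier write nothing.
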(fn SetRiverologyGES
  (params (Weather%20System%20-%20Wind%20Intensity :type Float%20%28double-precision%29) (Wind%20Strength%20Multiplier :type Float%20%28double-precision%29) (Wind%20Intensity%20Offset :type Float%20%28double-precision%29) (Wind%20Direction :type Float%20%28double-precision%29) (Wind%20Speed%20Struct :type Array%20of%20GES%20Riverology%20Wind%20Speed%20Struct%20Structures) (Use%20Wind%20Speed%20Array :type Boolean) (Weather%20Display%20Name%20Enum :type UDS_Weather_Display_Names%20Enum :default "NewEnumerator0"))
  (LocalVariables|SetWeather%20Display%20Name%20Enum%20Local Weather%20Display%20Name%20Enum)
  (LocalVariables|SetUse%20Wind%20Speed%20Array%20Local Use%20Wind%20Speed%20Array)
  (LocalVariables|SetWind%20Speed%20Struct%20Local Wind%20Speed%20Struct)
  (LocalVariables|SetWind%20Direction%20Local Wind%20Direction)
  (LocalVariables|SetWind%20Intensity%20Offset%20Local Wind%20Intensity%20Offset)
  (LocalVariables|SetWind%20Strength%20Multiplier%20Local Wind%20Strength%20Multiplier)
  (LocalVariables|SetWeather%20System%20Wind%20Intensity%20Local Weather%20System%20-%20Wind%20Intensity)
  (if (LocalVariables|GetUse%20Wind%20Speed%20Array%20Local)
    (Utilities|FlowControl|Sequence
      (:then_0
        ;[1 1 1] Weather Type Array
        (bind _array_element (Utilities|Array|ForEachLoopwithBreak (LocalVariables|GetWind%20Speed%20Struct%20Local) :!label _label)
          (:LoopBody
            (LocalVariables|SetDirection%20Offset1 (.directionoffset2 _array_element))
            (LocalVariables|SetDirection%20Offset (.directionoffset _array_element))
            (LocalVariables|SetDirection (.direction _array_element))
            (LocalVariables|SetWaveLength (.wavelength _array_element))
            (LocalVariables|SetSpeed (.speed _array_element))
            (LocalVariables|SetSteepness (.steepness _array_element))
            (LocalVariables|SetAmplitude (.amplitude _array_element))
            (LocalVariables|SetAmplitude_1 (.amplitude _array_element))
            (LocalVariables|SetSteepness_1 (.steepness_1 _array_element))
            (LocalVariables|SetSpeed_1 (.speed_1 _array_element))
            (LocalVariables|SetWaveLength_1 (.wavelength_1 _array_element))
            (LocalVariables|SetDirection_1 (.direction_1 _array_element))
            (LocalVariables|SetDirection_2 (.direction_2 _array_element))
            (LocalVariables|SetWaveLength_2 (.wavelength_2 _array_element))
            (LocalVariables|SetSpeed_2 (.speed_2 _array_element))
            (LocalVariables|SetSteepness_2 (.steepness_2 _array_element))
            (LocalVariables|SetAmplitude_2 (.amplitude_2 _array_element))
            (LocalVariables|SetAmplitude_3 (.amplitude_3 _array_element))
            (LocalVariables|SetSteepness_3 (.steepness_3 _array_element))
            (LocalVariables|SetSpeed_3 (.speed_3 _array_element))
            (LocalVariables|SetWaveLength_3 (.wavelength_3 _array_element))
            (LocalVariables|SetDirection_3 (.direction_3 _array_element))
            (LocalVariables|SetDirection_4 (.direction_4 _array_element))
            (LocalVariables|SetWaveLength_4 (.wavelength_4 _array_element))
            (LocalVariables|SetSpeed_4 (.speed_4 _array_element))
            (LocalVariables|SetSteepness_4 (.steepness_4 _array_element))
            (LocalVariables|SetAmplitude_4 (.amplitude_4 _array_element))
            (LocalVariables|SetPatchSize (.patchsize _array_element))
            (LocalVariables|SetCaustics%20Scale (.causticsscale _array_element))
            (LocalVariables|SetEdgeMask (.edgemask _array_element))
            (LocalVariables|SetChoppiness (.choppiness _array_element))
            (LocalVariables|SetGlobal%20Speed (.globalspeed _array_element))
            (LocalVariables|SetGlobal%20Amplitude (.globalamplitude _array_element))
            (LocalVariables|SetOverAllLength (.overalllength _array_element))
            (LocalVariables|SetArray%20Wind%20Speed%20Less%20Than (.windspeedlessthanequal _array_element))
            (LocalVariables|SetArray%20Wind%20Speed%20Greater%20Than (.windspeedgreaterthanequal _array_element))
            (LocalVariables|SetUse%20Multiplier (.usemultplier? _array_element))
            (LocalVariables|SetWeather%20Display%20Name%20Type%20Enum (.weathertypeenum _array_element))
            (LocalVariables|SetArray%20Use%20Display%20Name (.useweatherdisplayname? _array_element))
            (if (LocalVariables|GetArray%20Use%20Display%20Name)
              (if (Utilities|Enum|Equal(Enum) (LocalVariables|GetWeather%20Display%20Name%20Enum%20Local) (LocalVariables|GetWeather%20Display%20Name%20Type%20Enum))
                (if (not (LocalVariables|GetUse%20Multiplier)) :!label _label_2
                  ;;[0.875 0 1] Set Material Parameter Collection
                  (Rendering|Material|SetScalarParameterValue 0 "/Riverology_Plugin/Advanced/MaterialCollections/MPC_Riverology.MPC_Riverology" "Overall Length" (LocalVariables|GetOverAllLength) :!class /Script/Engine.KismetMaterialLibrary)
                  (Rendering|Material|SetScalarParameterValue 0 "/Riverology_Plugin/Advanced/MaterialCollections/MPC_Riverology.MPC_Riverology" "Global Amplitude" (LocalVariables|GetGlobal%20Amplitude) :!class /Script/Engine.KismetMaterialLibrary)
                  (Rendering|Material|SetScalarParameterValue 0 "/Riverology_Plugin/Advanced/MaterialCollections/MPC_Riverology.MPC_Riverology" "Global Speed" (LocalVariables|GetGlobal%20Speed) :!class /Script/Engine.KismetMaterialLibrary)
                  (Rendering|Material|SetScalarParameterValue 0 "/Riverology_Plugin/Advanced/MaterialCollections/MPC_Riverology.MPC_Riverology" "Choppiness" (LocalVariables|GetChoppiness) :!class /Script/Engine.KismetMaterialLibrary)
                  (Rendering|Material|SetScalarParameterValue 0 "/Riverology_Plugin/Advanced/MaterialCollections/MPC_Riverology.MPC_Riverology" "Direction_Offset_Σ" (LocalVariables|GetDirection%20Offset) :!class /Script/Engine.KismetMaterialLibrary)
                  (Rendering|Material|SetScalarParameterValue 0 "/Riverology_Plugin/Advanced/MaterialCollections/MPC_Riverology.MPC_Riverology" "Direction_Offset_Σ2" (LocalVariables|GetDirection%20Offset1) :!class /Script/Engine.KismetMaterialLibrary)
                  (Rendering|Material|SetScalarParameterValue 0 "/Riverology_Plugin/Advanced/MaterialCollections/MPC_Riverology.MPC_Riverology" "SIZE ( M )" (LocalVariables|GetPatchSize) :!class /Script/Engine.KismetMaterialLibrary)
                  (Rendering|Material|SetScalarParameterValue 0 "/Riverology_Plugin/Advanced/MaterialCollections/MPC_Riverology.MPC_Riverology" "EdgeMask" (LocalVariables|GetEdgeMask) :!class /Script/Engine.KismetMaterialLibrary)
                  (Rendering|Material|SetScalarParameterValue 0 "/Riverology_Plugin/Advanced/MaterialCollections/MPC_Riverology.MPC_Riverology" "Caustics Scale" (LocalVariables|GetCaustics%20Scale) :!class /Script/Engine.KismetMaterialLibrary)
                  (Rendering|Material|SetScalarParameterValue 0 "/Riverology_Plugin/Advanced/MaterialCollections/MPC_Riverology.MPC_Riverology" "Amplitude_Σ" (LocalVariables|GetAmplitude) :!class /Script/Engine.KismetMaterialLibrary)
                  (Rendering|Material|SetScalarParameterValue 0 "/Riverology_Plugin/Advanced/MaterialCollections/MPC_Riverology.MPC_Riverology" "Steepness_Σ" (LocalVariables|GetSteepness) :!class /Script/Engine.KismetMaterialLibrary)
                  (Rendering|Material|SetScalarParameterValue 0 "/Riverology_Plugin/Advanced/MaterialCollections/MPC_Riverology.MPC_Riverology" "Speed_Σ" (LocalVariables|GetSpeed) :!class /Script/Engine.KismetMaterialLibrary)
                  (Rendering|Material|SetScalarParameterValue 0 "/Riverology_Plugin/Advanced/MaterialCollections/MPC_Riverology.MPC_Riverology" "Wavelength_Σ" (LocalVariables|GetWaveLength) :!class /Script/Engine.KismetMaterialLibrary)
                  (Rendering|Material|SetScalarParameterValue 0 "/Riverology_Plugin/Advanced/MaterialCollections/MPC_Riverology.MPC_Riverology" "Direction_Σ" (LocalVariables|GetDirection) :!class /Script/Engine.KismetMaterialLibrary)
                  (Rendering|Material|SetScalarParameterValue 0 "/Riverology_Plugin/Advanced/MaterialCollections/MPC_Riverology.MPC_Riverology" "Amplitude_Σ1" (LocalVariables|GetAmplitude_1) :!class /Script/Engine.KismetMaterialLibrary)
                  (Rendering|Material|SetScalarParameterValue 0 "/Riverology_Plugin/Advanced/MaterialCollections/MPC_Riverology.MPC_Riverology" "Steepness_Σ1" (LocalVariables|GetSteepness_1) :!class /Script/Engine.KismetMaterialLibrary)
                  (Rendering|Material|SetScalarParameterValue 0 "/Riverology_Plugin/Advanced/MaterialCollections/MPC_Riverology.MPC_Riverology" "Speed_Σ1" (LocalVariables|GetSpeed_1) :!class /Script/Engine.KismetMaterialLibrary)
                  (Rendering|Material|SetScalarParameterValue 0 "/Riverology_Plugin/Advanced/MaterialCollections/MPC_Riverology.MPC_Riverology" "Wavelength_Σ1" (LocalVariables|GetWaveLength_1) :!class /Script/Engine.KismetMaterialLibrary)
                  (Rendering|Material|SetScalarParameterValue 0 "/Riverology_Plugin/Advanced/MaterialCollections/MPC_Riverology.MPC_Riverology" "Direction_Σ1" (LocalVariables|GetDirection_1) :!class /Script/Engine.KismetMaterialLibrary)
                  (Rendering|Material|SetScalarParameterValue 0 "/Riverology_Plugin/Advanced/MaterialCollections/MPC_Riverology.MPC_Riverology" "Amplitude_Σ2" (LocalVariables|GetAmplitude_2) :!class /Script/Engine.KismetMaterialLibrary)
                  (Rendering|Material|SetScalarParameterValue 0 "/Riverology_Plugin/Advanced/MaterialCollections/MPC_Riverology.MPC_Riverology" "Steepness_Σ2" (LocalVariables|GetSteepness_2) :!class /Script/Engine.KismetMaterialLibrary)
                  (Rendering|Material|SetScalarParameterValue 0 "/Riverology_Plugin/Advanced/MaterialCollections/MPC_Riverology.MPC_Riverology" "Speed_Σ2" (LocalVariables|GetSpeed_2) :!class /Script/Engine.KismetMaterialLibrary)
                  (Rendering|Material|SetScalarParameterValue 0 "/Riverology_Plugin/Advanced/MaterialCollections/MPC_Riverology.MPC_Riverology" "Wavelength_Σ2" (LocalVariables|GetWaveLength_2) :!class /Script/Engine.KismetMaterialLibrary)
                  (Rendering|Material|SetScalarParameterValue 0 "/Riverology_Plugin/Advanced/MaterialCollections/MPC_Riverology.MPC_Riverology" "Direction_Σ2" (LocalVariables|GetDirection_2) :!class /Script/Engine.KismetMaterialLibrary)
                  (Rendering|Material|SetScalarParameterValue 0 "/Riverology_Plugin/Advanced/MaterialCollections/MPC_Riverology.MPC_Riverology" "Amplitude_Σ3" (LocalVariables|GetAmplitude_3) :!class /Script/Engine.KismetMaterialLibrary)
                  (Rendering|Material|SetScalarParameterValue 0 "/Riverology_Plugin/Advanced/MaterialCollections/MPC_Riverology.MPC_Riverology" "Steepness_Σ3" (LocalVariables|GetSteepness_3) :!class /Script/Engine.KismetMaterialLibrary)
                  (Rendering|Material|SetScalarParameterValue 0 "/Riverology_Plugin/Advanced/MaterialCollections/MPC_Riverology.MPC_Riverology" "Speed_Σ3" (LocalVariables|GetSpeed_3) :!class /Script/Engine.KismetMaterialLibrary)
                  (Rendering|Material|SetScalarParameterValue 0 "/Riverology_Plugin/Advanced/MaterialCollections/MPC_Riverology.MPC_Riverology" "Wavelength_Σ3" (LocalVariables|GetWaveLength_3) :!class /Script/Engine.KismetMaterialLibrary)
                  (Rendering|Material|SetScalarParameterValue 0 "/Riverology_Plugin/Advanced/MaterialCollections/MPC_Riverology.MPC_Riverology" "Direction_Σ3" (LocalVariables|GetDirection_3) :!class /Script/Engine.KismetMaterialLibrary)
                  (Rendering|Material|SetScalarParameterValue 0 "/Riverology_Plugin/Advanced/MaterialCollections/MPC_Riverology.MPC_Riverology" "Amplitude_Σ4" (LocalVariables|GetAmplitude_4) :!class /Script/Engine.KismetMaterialLibrary)
                  (Rendering|Material|SetScalarParameterValue 0 "/Riverology_Plugin/Advanced/MaterialCollections/MPC_Riverology.MPC_Riverology" "Steepness_Σ4" (LocalVariables|GetSteepness_4) :!class /Script/Engine.KismetMaterialLibrary)
                  (Rendering|Material|SetScalarParameterValue 0 "/Riverology_Plugin/Advanced/MaterialCollections/MPC_Riverology.MPC_Riverology" "Speed_Σ4" (LocalVariables|GetSpeed_4) :!class /Script/Engine.KismetMaterialLibrary)
                  (Rendering|Material|SetScalarParameterValue 0 "/Riverology_Plugin/Advanced/MaterialCollections/MPC_Riverology.MPC_Riverology" "Wavelength_Σ4" (LocalVariables|GetWaveLength_4) :!class /Script/Engine.KismetMaterialLibrary)
                  (Rendering|Material|SetScalarParameterValue 0 "/Riverology_Plugin/Advanced/MaterialCollections/MPC_Riverology.MPC_Riverology" "Direction_Σ4" (LocalVariables|GetDirection_4) :!class /Script/Engine.KismetMaterialLibrary)
                  (goto _label Break)))
              (elif (Math|Float|InRange(Float) (LocalVariables|GetWeather%20System%20Wind%20Intensity%20Local) (LocalVariables|GetArray%20Wind%20Speed%20Greater%20Than) (LocalVariables|GetArray%20Wind%20Speed%20Less%20Than))
                (goto _label_2)))))))
    (else
      (Utilities|FlowControl|Sequence
        (:then_0
          ;[0 0.01562 1] Adjust Wind Speed
          (LocalVariables|SetWind%20Intensity%20Adjusted%20Local (+ (* (LocalVariables|GetWeather%20System%20Wind%20Intensity%20Local) (LocalVariables|GetWind%20Strength%20Multiplier%20Local)) (LocalVariables|GetWind%20Intensity%20Offset%20Local))))
        (:then_1
          ;[0.875 0 1] Set Material Parameter Collection Globals
          (Rendering|Material|SetScalarParameterValue 0 "/Riverology_Plugin/Advanced/MaterialCollections/MPC_Riverology.MPC_Riverology" "Global Amplitude" (LocalVariables|GetWind%20Intensity%20Adjusted%20Local) :!class /Script/Engine.KismetMaterialLibrary)
          (Rendering|Material|SetScalarParameterValue 0 "/Riverology_Plugin/Advanced/MaterialCollections/MPC_Riverology.MPC_Riverology" "Global Speed" (LocalVariables|GetWind%20Intensity%20Adjusted%20Local) :!class /Script/Engine.KismetMaterialLibrary))))))