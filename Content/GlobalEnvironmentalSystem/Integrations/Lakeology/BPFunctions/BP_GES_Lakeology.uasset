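; Function library that links the Global Environmental System weather to Oceanology lake waves.
; SetLakeologyGES matches entries in a wind-speed array by weather name or intensity range, then applies a lake preset or writes per-wave MPC_Waves parameters, skipping unchanged presets or amplitude.
; Without the array, wind intensity directly drives global amplitude and speed.
; A previously stored direction-change flag short-circuits to updating only wave direction from the stored value.
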(fn SetLakeologyGES
  (params (Weather%20System%20-%20Wind%20Intensity :type Float%20%28double-precision%29) (Wind%20Direction :type Float%20%28double-precision%29) (Wind%20Speed%20Struct :type Array%20of%20GES%20Lakeology%20Wind%20Speed%20Struct%20Structures) (Weather%20Display%20Name%20Enum :type GES_UDS_Weather_Display_Names%20Enum :default "NewEnumerator0") (Wind%20Direction%20Change :type Boolean) (Use%20Wind%20Speed%20Array :type Boolean))
  ;[1 1 1] Comment
  (if (LocalVariables|GetWind%20Direction%20Change%20Local)
    ;;[1 1 1] Direcrtion
    (Rendering|Material|SetScalarParameterValue 0 "/Oceanology_Plugin/Design/Ocean/MaterialCollections/MPC_Waves.MPC_Waves" "GlobalWaveDirection" (LocalVariables|GetWind%20Direction%20Local) :!class /Script/Engine.KismetMaterialLibrary)
    (else
      (LocalVariables|SetUse%20Wind%20Speed%20Array%20Local Use%20Wind%20Speed%20Array)
      (bind _returnvalue (Actor|GetActorOfClass 0 "/Oceanology_Plugin/Design/Lake/Blueprints/Lake/BP_OceanologyLake.BP_OceanologyLake_C"))
      (LocalVariables|SetLakeology%20BP _returnvalue)
      (LocalVariables|SetWind%20Direction%20Change%20Local Wind%20Direction%20Change)
      (LocalVariables|SetWeather%20Display%20Name%20Enum%20Local Weather%20Display%20Name%20Enum)
      (LocalVariables|SetWind%20Speed%20Struct%20Local Wind%20Speed%20Struct)
      (LocalVariables|SetWind%20Direction%20Local Wind%20Direction)
      (LocalVariables|SetWeather%20System%20Wind%20Intensity%20Local Weather%20System%20-%20Wind%20Intensity)
      (if (LocalVariables|GetUse%20Wind%20Speed%20Array%20Local)
        (bind _array_element (Utilities|Array|ForEachLoopwithBreak (LocalVariables|GetWind%20Speed%20Struct%20Local) :!label _label)
          (:LoopBody
            (bind _returnvalue_2 (Utilities|LoadAssetBlocking (.lakepreset _array_element)))
            (bind _asoceanology_lake_preset (Utilities|Casting|CastToOceanologyLakePreset _returnvalue_2))
            (LocalVariables|SetArray%20Lake%20Preset _asoceanology_lake_preset)
            (LocalVariables|SetDirection%20Offset2 (.directionoffset2 _array_element))
            (LocalVariables|SetDirection%20Offset (.directionoffset _array_element))
            (LocalVariables|SetDirection (.direction _array_element))
            (LocalVariables|SetWaveLength (.wavelength _array_element))
            (LocalVariables|SetSpeed (.speed _array_element))
            (LocalVariables|SetSteepness (.steepness _array_element))
            (LocalVariables|SetAmplitude (.amplitude _array_element))
            (LocalVariables|SetAmplitude_1 (.amplitude _array_element))
            (LocalVariables|SetSteepness_1 (.steepness_1 _array_element))
            (LocalVariables|SetSpeed_1 (.speed_1 _array_element))
            (LocalVariables|SetWaveLength_1 (.wavelength_1 _array_element))
            (LocalVariables|SetDirection_1 (.direction_1 _array_element))
            (LocalVariables|SetDirection_2 (.direction_2 _array_element))
            (LocalVariables|SetWaveLength_2 (.wavelength_2 _array_element))
            (LocalVariables|SetSpeed_2 (.speed_2 _array_element))
            (LocalVariables|SetSteepness_2 (.steepness_2 _array_element))
            (LocalVariables|SetAmplitude_2 (.amplitude_2 _array_element))
            (LocalVariables|SetAmplitude_3 (.amplitude_3 _array_element))
            (LocalVariables|SetSteepness_3 (.steepness_3 _array_element))
            (LocalVariables|SetSpeed_3 (.speed_3 _array_element))
            (LocalVariables|SetWaveLength_3 (.wavelength_3 _array_element))
            (LocalVariables|SetDirection_3 (.direction_3 _array_element))
            (LocalVariables|SetDirection_4 (.direction_4 _array_element))
            (LocalVariables|SetWaveLength_4 (.wavelength_4 _array_element))
            (LocalVariables|SetSpeed_4 (.speed_4 _array_element))
            (LocalVariables|SetSteepness_4 (.steepness_4 _array_element))
            (LocalVariables|SetAmplitude_4 (.amplitude_4 _array_element))
            (LocalVariables|SetPatchSize (.patchsize _array_element))
            (LocalVariables|SetGlobal%20Wave%20Direction (.globalwavedirection _array_element))
            (LocalVariables|SetChoppiness (.choppiness _array_element))
            (LocalVariables|SetGlobal%20Speed (.globalspeed _array_element))
            (LocalVariables|SetGlobal%20Amplitude (.globalamplitude _array_element))
            (LocalVariables|SetOverAllLength (.overalllength _array_element))
            (LocalVariables|SetArray%20Wind%20Speed%20Less%20Than (.windspeedlessthanequal _array_element))
            (LocalVariables|SetArray%20Wind%20Speed%20Greater%20Than (.windspeedgreaterthanequal _array_element))
            (LocalVariables|SetUse%20Lake%20Preset (.uselakepreset? _array_element))
            (LocalVariables|SetUse%20Multiplier (.usemultplier? _array_element))
            (LocalVariables|SetWeather%20Display%20Name%20Type%20Enum (.weathertypeenum _array_element))
            (LocalVariables|SetArray%20Use%20Display%20Name (.useweatherdisplayname? _array_element))
            (if (LocalVariables|GetArray%20Use%20Display%20Name)
              (if (Utilities|Enum|Equal(Enum) (LocalVariables|GetWeather%20Display%20Name%20Enum%20Local) (LocalVariables|GetWeather%20Display%20Name%20Type%20Enum))
                (if (LocalVariables|GetUse%20Multiplier) :!label _label_2
                  _
                  (else
                    _))
                (if (LocalVariables|GetUse%20Lake%20Preset)
                  ;;[0.1787 0.2838 1] Use Preset
                  (if (!= (Variables|/Script/Oceanology_Plugin.OceanologyLake|GetPreset (LocalVariables|GetLakeology%20BP)) (LocalVariables|GetArray%20Lake%20Preset))
                    (Variables|/Script/Oceanology_Plugin.OceanologyLake|SetPreset (LocalVariables|GetLakeology%20BP) (LocalVariables|GetArray%20Lake%20Preset))
                    (Class|OceanologyWaterParent|ReloadSettings (LocalVariables|GetLakeology%20BP))
                    (goto _label Break))
                  (else
                    (bind _returnvalue_3 (Rendering|Material|GetScalarParameterValue 0 "/Oceanology_Plugin/Design/Ocean/MaterialCollections/MPC_Waves.MPC_Waves" "Amplitude" :!class /Script/Engine.KismetMaterialLibrary))
                    (if (!= _returnvalue_3 (LocalVariables|GetAmplitude))
                      ;;[0.875 0 1] Set Material Parameter Collection
                      (Rendering|Material|SetScalarParameterValue 0 "/Oceanology_Plugin/Design/Ocean/MaterialCollections/MPC_Waves.MPC_Waves" "Overall Length" (LocalVariables|GetOverAllLength) :!class /Script/Engine.KismetMaterialLibrary)
                      (Rendering|Material|SetScalarParameterValue 0 "/Oceanology_Plugin/Design/Ocean/MaterialCollections/MPC_Waves.MPC_Waves" "Global Amplitude" (LocalVariables|GetGlobal%20Amplitude) :!class /Script/Engine.KismetMaterialLibrary)
                      (Rendering|Material|SetScalarParameterValue 0 "/Oceanology_Plugin/Design/Ocean/MaterialCollections/MPC_Waves.MPC_Waves" "Global Speed" (LocalVariables|GetGlobal%20Speed) :!class /Script/Engine.KismetMaterialLibrary)
                      (Rendering|Material|SetScalarParameterValue 0 "/Oceanology_Plugin/Design/Ocean/MaterialCollections/MPC_Waves.MPC_Waves" "Choppiness" (LocalVariables|GetChoppiness) :!class /Script/Engine.KismetMaterialLibrary)
                      (Rendering|Material|SetScalarParameterValue 0 "/Oceanology_Plugin/Design/Ocean/MaterialCollections/MPC_Waves.MPC_Waves" "GlobalWaveDirection" (LocalVariables|GetWind%20Direction%20Local) :!class /Script/Engine.KismetMaterialLibrary)
                      (Rendering|Material|SetScalarParameterValue 0 "/Oceanology_Plugin/Design/Ocean/MaterialCollections/MPC_Waves.MPC_Waves" "Direction_Offset" (LocalVariables|GetDirection%20Offset) :!class /Script/Engine.KismetMaterialLibrary)
                      (Rendering|Material|SetScalarParameterValue 0 "/Oceanology_Plugin/Design/Ocean/MaterialCollections/MPC_Waves.MPC_Waves" "Direction_Offset_2" (LocalVariables|GetDirection%20Offset2) :!class /Script/Engine.KismetMaterialLibrary)
                      (Rendering|Material|SetScalarParameterValue 0 "/Oceanology_Plugin/Design/Ocean/MaterialCollections/MPC_Waves.MPC_Waves" "PatchSize" (LocalVariables|GetPatchSize) :!class /Script/Engine.KismetMaterialLibrary)
                      (Rendering|Material|SetScalarParameterValue 0 "/Oceanology_Plugin/Design/Ocean/MaterialCollections/MPC_Waves.MPC_Waves" "Amplitude" (LocalVariables|GetAmplitude) :!class /Script/Engine.KismetMaterialLibrary)
                      (Rendering|Material|SetScalarParameterValue 0 "/Oceanology_Plugin/Design/Ocean/MaterialCollections/MPC_Waves.MPC_Waves" "Steepness" (LocalVariables|GetSteepness) :!class /Script/Engine.KismetMaterialLibrary)
                      (Rendering|Material|SetScalarParameterValue 0 "/Oceanology_Plugin/Design/Ocean/MaterialCollections/MPC_Waves.MPC_Waves" "Speed" (LocalVariables|GetSpeed) :!class /Script/Engine.KismetMaterialLibrary)
                      (Rendering|Material|SetScalarParameterValue 0 "/Oceanology_Plugin/Design/Ocean/MaterialCollections/MPC_Waves.MPC_Waves" "Wavelength" (LocalVariables|GetWaveLength) :!class /Script/Engine.KismetMaterialLibrary)
                      (Rendering|Material|SetScalarParameterValue 0 "/Oceanology_Plugin/Design/Ocean/MaterialCollections/MPC_Waves.MPC_Waves" "Direction" (LocalVariables|GetDirection) :!class /Script/Engine.KismetMaterialLibrary)
                      (Rendering|Material|SetScalarParameterValue 0 "/Oceanology_Plugin/Design/Ocean/MaterialCollections/MPC_Waves.MPC_Waves" "Amplitude_1" (LocalVariables|GetAmplitude_1) :!class /Script/Engine.KismetMaterialLibrary)
                      (Rendering|Material|SetScalarParameterValue 0 "/Oceanology_Plugin/Design/Ocean/MaterialCollections/MPC_Waves.MPC_Waves" "Steepness_1" (LocalVariables|GetSteepness_1) :!class /Script/Engine.KismetMaterialLibrary)
                      (Rendering|Material|SetScalarParameterValue 0 "/Oceanology_Plugin/Design/Ocean/MaterialCollections/MPC_Waves.MPC_Waves" "Speed_1" (LocalVariables|GetSpeed_1) :!class /Script/Engine.KismetMaterialLibrary)
                      (Rendering|Material|SetScalarParameterValue 0 "/Oceanology_Plugin/Design/Ocean/MaterialCollections/MPC_Waves.MPC_Waves" "Wavelength_1" (LocalVariables|GetWaveLength_1) :!class /Script/Engine.KismetMaterialLibrary)
                      (Rendering|Material|SetScalarParameterValue 0 "/Oceanology_Plugin/Design/Ocean/MaterialCollections/MPC_Waves.MPC_Waves" "Direction_1" (LocalVariables|GetDirection_1) :!class /Script/Engine.KismetMaterialLibrary)
                      (Rendering|Material|SetScalarParameterValue 0 "/Oceanology_Plugin/Design/Ocean/MaterialCollections/MPC_Waves.MPC_Waves" "Amplitude_2" (LocalVariables|GetAmplitude_2) :!class /Script/Engine.KismetMaterialLibrary)
                      (Rendering|Material|SetScalarParameterValue 0 "/Oceanology_Plugin/Design/Ocean/MaterialCollections/MPC_Waves.MPC_Waves" "Steepness_2" (LocalVariables|GetSteepness_2) :!class /Script/Engine.KismetMaterialLibrary)
                      (Rendering|Material|SetScalarParameterValue 0 "/Oceanology_Plugin/Design/Ocean/MaterialCollections/MPC_Waves.MPC_Waves" "Speed_2" (LocalVariables|GetSpeed_2) :!class /Script/Engine.KismetMaterialLibrary)
                      (Rendering|Material|SetScalarParameterValue 0 "/Oceanology_Plugin/Design/Ocean/MaterialCollections/MPC_Waves.MPC_Waves" "Wavelength_2" (LocalVariables|GetWaveLength_2) :!class /Script/Engine.KismetMaterialLibrary)
                      (Rendering|Material|SetScalarParameterValue 0 "/Oceanology_Plugin/Design/Ocean/MaterialCollections/MPC_Waves.MPC_Waves" "Direction_2" (LocalVariables|GetDirection_2) :!class /Script/Engine.KismetMaterialLibrary)
                      (Rendering|Material|SetScalarParameterValue 0 "/Oceanology_Plugin/Design/Ocean/MaterialCollections/MPC_Waves.MPC_Waves" "Amplitude_3" (LocalVariables|GetAmplitude_3) :!class /Script/Engine.KismetMaterialLibrary)
                      (Rendering|Material|SetScalarParameterValue 0 "/Oceanology_Plugin/Design/Ocean/MaterialCollections/MPC_Waves.MPC_Waves" "Steepness_3" (LocalVariables|GetSteepness_3) :!class /Script/Engine.KismetMaterialLibrary)
                      (Rendering|Material|SetScalarParameterValue 0 "/Oceanology_Plugin/Design/Ocean/MaterialCollections/MPC_Waves.MPC_Waves" "Speed_3" (LocalVariables|GetSpeed_3) :!class /Script/Engine.KismetMaterialLibrary)
                      (Rendering|Material|SetScalarParameterValue 0 "/Oceanology_Plugin/Design/Ocean/MaterialCollections/MPC_Waves.MPC_Waves" "Wavelength_3" (LocalVariables|GetWaveLength_3) :!class /Script/Engine.KismetMaterialLibrary)
                      (Rendering|Material|SetScalarParameterValue 0 "/Oceanology_Plugin/Design/Ocean/MaterialCollections/MPC_Waves.MPC_Waves" "Direction_3" (LocalVariables|GetDirection_3) :!class /Script/Engine.KismetMaterialLibrary)
                      (Rendering|Material|SetScalarParameterValue 0 "/Oceanology_Plugin/Design/Ocean/MaterialCollections/MPC_Waves.MPC_Waves" "Amplitude_4" (LocalVariables|GetAmplitude_4) :!class /Script/Engine.KismetMaterialLibrary)
                      (Rendering|Material|SetScalarParameterValue 0 "/Oceanology_Plugin/Design/Ocean/MaterialCollections/MPC_Waves.MPC_Waves" "Steepness_4" (LocalVariables|GetSteepness_4) :!class /Script/Engine.KismetMaterialLibrary)
                      (Rendering|Material|SetScalarParameterValue 0 "/Oceanology_Plugin/Design/Ocean/MaterialCollections/MPC_Waves.MPC_Waves" "Speed_4" (LocalVariables|GetSpeed_4) :!class /Script/Engine.KismetMaterialLibrary)
                      (Rendering|Material|SetScalarParameterValue 0 "/Oceanology_Plugin/Design/Ocean/MaterialCollections/MPC_Waves.MPC_Waves" "Wavelength_4" (LocalVariables|GetWaveLength_4) :!class /Script/Engine.KismetMaterialLibrary)
                      (Rendering|Material|SetScalarParameterValue 0 "/Oceanology_Plugin/Design/Ocean/MaterialCollections/MPC_Waves.MPC_Waves" "Direction_4" (LocalVariables|GetDirection_4) :!class /Script/Engine.KismetMaterialLibrary)
                      (goto _label Break)))))
              (elif (Math|Float|InRange(Float) (LocalVariables|GetWeather%20System%20Wind%20Intensity%20Local) (LocalVariables|GetArray%20Wind%20Speed%20Greater%20Than) (LocalVariables|GetArray%20Wind%20Speed%20Less%20Than))
                (goto _label_2)))))
        (else
          ;;[0.875 0 1] Set Material Parameter Collection Globals
          (Rendering|Material|SetScalarParameterValue 0 "/Oceanology_Plugin/Design/Ocean/MaterialCollections/MPC_Waves.MPC_Waves" "Global Amplitude" (LocalVariables|GetWeather%20System%20Wind%20Intensity%20Local) :!class /Script/Engine.KismetMaterialLibrary)
          (Rendering|Material|SetScalarParameterValue 0 "/Oceanology_Plugin/Design/Ocean/MaterialCollections/MPC_Waves.MPC_Waves" "Global Speed" (LocalVariables|GetWeather%20System%20Wind%20Intensity%20Local) :!class /Script/Engine.KismetMaterialLibrary))))))