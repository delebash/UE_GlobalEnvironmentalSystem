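; Global Environmental System integration that drives Mawi wind by writing weather data into the MPC_MW_Controller material parameter collection.
; SetMawiGES always sets wind direction, then either passes weather wind intensity through with a fixed speed or searches a wind array.
; Array entries match by weather type or intensity range, optionally scale by a strength multiplier, and stop the search once applied.
; Range matches write only when the current intensity differs.
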(fn SetMawiGES
  (params (Weather%20System%20-%20Wind%20Intensity :type Float%20%28double-precision%29) (Wind%20Strength%20Multiplier :type Float%20%28double-precision%29) (Wind%20Speed%20Array :type Array%20of%20GES%20Mawi%20Wind%20Speed%20Struct%20Structures) (Weather%20Display%20Name%20Enum :type GES_UDS_Weather_Display_Names%20Enum :default "NewEnumerator15") (Use%20Wind%20Speed%20Array :type Boolean) (Wind%20Direction%20Vector :type Vector))
  (LocalVariables|SetWeather%20System%20Wind%20Intensity%20Local Weather%20System%20-%20Wind%20Intensity)
  (LocalVariables|SetWind%20Strength%20Multiplier%20Local Wind%20Strength%20Multiplier)
  (LocalVariables|SetWind%20Speed%20Array%20Local Wind%20Speed%20Array)
  (LocalVariables|SetWeather%20Display%20Name%20Enum%20Local Weather%20Display%20Name%20Enum)
  (LocalVariables|SetUse%20Wind%20Speed%20Array%20Local Use%20Wind%20Speed%20Array)
  (LocalVariables|SetWind%20Direction%20Vector%20Local Wind%20Direction%20Vector)
  (Utilities|FlowControl|Sequence
    (:then_0
      ;[1 1 1] Wind Direction
      (Rendering|Material|SetVectorParameterValue 0 "/Game/MWCommon/_Legacy/Materials/MASTER/Par/MPC_MW_Controller.MPC_MW_Controller" "MW_WindDirection" (Math|Conversions|ToLinearColor(Vector) (LocalVariables|GetWind%20Direction%20Vector%20Local)) :!class /Script/Engine.KismetMaterialLibrary))
    (:then_1
      ;[1 1 1] Weather Type Wind Speed Array
      (if (LocalVariables|GetUse%20Wind%20Speed%20Array%20Local)
        (bind _array_element (Utilities|Array|ForEachLoopwithBreak (LocalVariables|GetWind%20Speed%20Array%20Local) :!label _label)
          (:LoopBody
            (LocalVariables|SetArray%20Wind%20Intensity (.windintensity _array_element))
            (LocalVariables|SetArray%20Wind%20Speed (.windspeed _array_element))
            (LocalVariables|SetArray%20Wind%20Speed%20Less%20Than (.windspeedlessthanequal _array_element))
            (LocalVariables|SetArray%20Use%20Multiplier (.usemultplier? _array_element))
            (LocalVariables|SetArray%20Wind%20Speed%20Greater%20Than (.windspeedgreaterthanequal _array_element))
            (LocalVariables|SetArray%20Weather%20Display%20Name%20Type%20Enum (.weathertypeenum _array_element))
            (if (.useweathernameorvalue _array_element)
              (if (Utilities|Enum|Equal(Enum) (LocalVariables|GetWeather%20Display%20Name%20Enum%20Local) (LocalVariables|GetArray%20Weather%20Display%20Name%20Type%20Enum))
                (if (LocalVariables|GetArray%20Use%20Multiplier) :!label _label_2
                  (LocalVariables|SetArray%20Wind%20Intensity (* (LocalVariables|GetWind%20Strength%20Multiplier%20Local) (LocalVariables|GetArray%20Wind%20Intensity)))
                  (LocalVariables|SetArray%20Wind%20Speed (* (LocalVariables|GetWind%20Strength%20Multiplier%20Local) (LocalVariables|GetArray%20Wind%20Speed))))
                ;[0.1995 0.2653 1] Mawi Wind Parameters
                (Rendering|Material|SetScalarParameterValue 0 "/Game/MWCommon/_Legacy/Materials/MASTER/Par/MPC_MW_Controller.MPC_MW_Controller" "MW_WindIntensity" (LocalVariables|GetArray%20Wind%20Intensity) :!class /Script/Engine.KismetMaterialLibrary)
                (Rendering|Material|SetScalarParameterValue 0 "/Game/MWCommon/_Legacy/Materials/MASTER/Par/MPC_MW_Controller.MPC_MW_Controller" "MW_WindSpeed" (LocalVariables|GetArray%20Wind%20Speed) :!class /Script/Engine.KismetMaterialLibrary)
                (goto _label Break))
              (elif (Math|Float|InRange(Float) (LocalVariables|GetWeather%20System%20Wind%20Intensity%20Local) (LocalVariables|GetArray%20Wind%20Speed%20Greater%20Than) (LocalVariables|GetArray%20Wind%20Speed%20Less%20Than))
                (bind _returnvalue (Rendering|Material|GetScalarParameterValue 0 "/Game/MWCommon/_Legacy/Materials/MASTER/Par/MPC_MW_Controller.MPC_MW_Controller" "MW_WindIntensity" :!class /Script/Engine.KismetMaterialLibrary))
                (if (!= _returnvalue (LocalVariables|GetArray%20Wind%20Intensity))
                  (goto _label_2))))))
        (else
          ;[0.1995 0.2653 1] Mawi Wind Parameters
          (Rendering|Material|SetScalarParameterValue 0 "/Game/MWCommon/_Legacy/Materials/MASTER/Par/MPC_MW_Controller.MPC_MW_Controller" "MW_WindSpeed" 1.5 :!class /Script/Engine.KismetMaterialLibrary)
          (Rendering|Material|SetScalarParameterValue 0 "/Game/MWCommon/_Legacy/Materials/MASTER/Par/MPC_MW_Controller.MPC_MW_Controller" "MW_WindIntensity" (LocalVariables|GetWeather%20System%20Wind%20Intensity%20Local) :!class /Script/Engine.KismetMaterialLibrary))))))