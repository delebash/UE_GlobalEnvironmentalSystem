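; Blueprint function that serves as a reference integration between a weather system's wind and the Global Environmental System (GES).
; SetReferenceGES scales the incoming wind intensity by a strength multiplier and adds an offset.
; It writes the result to the "Wind Strength" scalar of a Material Parameter Collection.
; Wind direction is accepted and stored locally but never applied.
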(fn SetReferenceGES
  (params (Weather%20System%20-%20Wind%20Intensity :type Float%20%28double-precision%29) (Wind%20Strength%20Multiplier :type Float%20%28double-precision%29) (Wind%20Intensity%20Offset :type Float%20%28double-precision%29) (Wind%20Direction :type Float%20%28double-precision%29))
  (LocalVariables|SetWind%20Direction%20Local Wind%20Direction)
  (LocalVariables|SetWind%20Intensity%20Offset%20Local Wind%20Intensity%20Offset)
  (LocalVariables|SetWind%20Strength%20Multiplier%20Local Wind%20Strength%20Multiplier)
  (LocalVariables|SetWeather%20System%20Wind%20Intensity%20Local Weather%20System%20-%20Wind%20Intensity)
  (Utilities|FlowControl|Sequence
    (:then_0
      ;[0 0.01562 1] Adjust Wind Speed
      (LocalVariables|SetWind%20Intensity%20Adjusted%20Local (+ (* (LocalVariables|GetWeather%20System%20Wind%20Intensity%20Local) (LocalVariables|GetWind%20Strength%20Multiplier%20Local)) (LocalVariables|GetWind%20Intensity%20Offset%20Local))))
    (:then_1
      ;[0.875 0 1] Set Material Parameter Collection
      (Rendering|Material|SetScalarParameterValue 0 0 "Wind Strength" (LocalVariables|GetWind%20Intensity%20Adjusted%20Local) :!class /Script/Engine.KismetMaterialLibrary))))